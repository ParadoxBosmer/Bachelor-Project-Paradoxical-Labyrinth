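; BP_Camera is a camera pickup actor that the player can collect.
; Overlap events on its Trigger component show and hide a Widget component, and a custom event also hides it.
; The Interact event casts the player character to BP_FirstPersonCharacter, passes "Camera" to PickUpItem, then destroys the actor.
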(event `CustomEvent`
  (`SceneComponent.SetHiddenInGame` (`self.Widget`) true false))

(event `self.Trigger.OnComponentBeginOverlap`
  (params (OverlappedComponent :type "PrimitiveComponent Object Reference") (OtherActor :type "Actor Object Reference") (OtherComp :type "PrimitiveComponent Object Reference") (OtherBodyIndex :type Integer) (bFromSweep :type Boolean) (SweepResult :type "HitResult Structure (by ref)"))
  (`SceneComponent.SetHiddenInGame` (`self.Widget`) false false))

(event `self.Trigger.OnComponentEndOverlap`
  (params (OverlappedComponent :type "PrimitiveComponent Object Reference") (OtherActor :type "Actor Object Reference") (OtherComp :type "PrimitiveComponent Object Reference") (OtherBodyIndex :type Integer))
  (`SceneComponent.SetHiddenInGame` (`self.Widget`) true false))

(event `/Game/Blueprints/BPI_Interaction.Interact`
  (bind _asbp_first_person_character (cast `/Game/ThirdPerson/Blueprints/BP_FirstPersonCharacter` (`GameplayStatics.GetPlayerCharacter` 0)))
  (`/Game/ThirdPerson/Blueprints/BP_FirstPersonCharacter.Pick up Item` _asbp_first_person_character "Camera")
  (`self.K2_DestroyActor`))

(fn `UserConstructionScript`)