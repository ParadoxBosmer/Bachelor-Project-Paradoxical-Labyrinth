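; BP_Door_True is the correct door actor that ends the game with a win when interacted with.
; A trigger volume shows a prompt widget while something overlaps it and hides it on exit.
; Interact waits briefly, adds the WB_Win screen to the viewport if the player is the first-person character, then disables input and pauses the game.
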(event `self.Trigger.OnComponentBeginOverlap`
  (params (OverlappedComponent :type "PrimitiveComponent Object Reference") (OtherActor :type "Actor Object Reference") (OtherComp :type "PrimitiveComponent Object Reference") (OtherBodyIndex :type Integer) (bFromSweep :type Boolean) (SweepResult :type "HitResult Structure (by ref)"))
  (`SceneComponent.SetHiddenInGame` (`self.Widget`) false false))

(event `self.Trigger.OnComponentEndOverlap`
  (params (OverlappedComponent :type "PrimitiveComponent Object Reference") (OtherActor :type "Actor Object Reference") (OtherComp :type "PrimitiveComponent Object Reference") (OtherBodyIndex :type Integer))
  (`SceneComponent.SetHiddenInGame` (`self.Widget`) true false))

(event `/Game/Blueprints/BPI_Interaction.Interact`
  (`KismetSystemLibrary.Delay` 0.2)
  (bind _returnvalue (`|CreateWidget` "/Game/UI/WB_Win.WB_Win_C"))
  (cast `/Game/ThirdPerson/Blueprints/BP_FirstPersonCharacter` (`GameplayStatics.GetPlayerCharacter` 0))
  (`UserWidget.AddToViewport` _returnvalue 0)
  (`self.DisableInput` null)
  (`GameplayStatics.SetGamePaused` true))

(fn `UserConstructionScript`)